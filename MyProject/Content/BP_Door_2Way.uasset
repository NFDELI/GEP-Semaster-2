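; BP_Door_2Way is an automatic double door that swings in either direction depending on which trigger, Front or Back, is overlapped first.
; That overlap records the swing side, disables the opposite trigger's collision and plays the DoorSwing timeline, which rotates both leaves in mirrored yaw with sweep.
; Ending the overlap reverses the timeline, and a completed close clears the open state and re-enables both triggers for queries.
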(event OnComponentBeginOverlap(Front)
  (params (OverlappedComponent :type Primitive%20Component%20Object%20Reference) (OtherActor :type Actor%20Object%20Reference) (OtherComp :type Primitive%20Component%20Object%20Reference) (OtherBodyIndex :type Integer) (bFromSweep :type Boolean) (SweepResult :type Hit%20Result%20Structure%20%28by%20ref%29))
  (if (Variables|Default|Getm_bOpen)
    (if (Variables|Default|Getm_bSwingFront)
      (Collision|SetCollisionEnabled (Variables|Default|GetBack) "NoCollision" :!label _label)
      ;[1 1 1] Door Openning
      (bind (_direction _delta) (Timeline|DoorSwing Play)
        (:Update
          (Transformation|SetRelativeRotation (Variables|Default|GetDoor2) (Math|Rotator|MakeRotator 0.0 0.0 (* _delta (Variables|Default|Getm_fSwingRotTarget) (Math|Float|SelectFloat 1.0 -1.0 (Variables|Default|Getm_bSwingFront)))) true false)
          (Transformation|SetRelativeRotation (Variables|Default|GetDoor1) (* (Math|Rotator|MakeRotator 0.0 0.0 (* _delta (Variables|Default|Getm_fSwingRotTarget) (Math|Float|SelectFloat 1.0 -1.0 (Variables|Default|Getm_bSwingFront)))) -1.0) true false))
        (:Finished
          (if (Utilities|Enum|Equal(Enum) _direction "Backward")
            (Variables|Default|Setm_bOpen false)
            (Collision|SetCollisionEnabled (Variables|Default|GetFront) "QueryOnly")))))
    (else
      (Variables|Default|Setm_bSwingFront true)
      (Variables|Default|Setm_bOpen true)
      (goto _label))))

(event OnComponentEndOverlap(Front)
  (params (OverlappedComponent :type Primitive%20Component%20Object%20Reference) (OtherActor :type Actor%20Object%20Reference) (OtherComp :type Primitive%20Component%20Object%20Reference) (OtherBodyIndex :type Integer))
  ;[1 1 1] Door Openning
  (bind (_direction _delta) (Timeline|DoorSwing Reverse)
    (:Update
      (Transformation|SetRelativeRotation (Variables|Default|GetDoor2) (Math|Rotator|MakeRotator 0.0 0.0 (* _delta (Variables|Default|Getm_fSwingRotTarget) (Math|Float|SelectFloat 1.0 -1.0 (Variables|Default|Getm_bSwingFront)))) true false)
      (Transformation|SetRelativeRotation (Variables|Default|GetDoor1) (* (Math|Rotator|MakeRotator 0.0 0.0 (* _delta (Variables|Default|Getm_fSwingRotTarget) (Math|Float|SelectFloat 1.0 -1.0 (Variables|Default|Getm_bSwingFront)))) -1.0) true false))
    (:Finished
      (if (Utilities|Enum|Equal(Enum) _direction "Backward")
        (Variables|Default|Setm_bOpen false)
        (Collision|SetCollisionEnabled (Variables|Default|GetFront) "QueryOnly")))))

(event OnComponentBeginOverlap(Back)
  (params (OverlappedComponent :type Primitive%20Component%20Object%20Reference) (OtherActor :type Actor%20Object%20Reference) (OtherComp :type Primitive%20Component%20Object%20Reference) (OtherBodyIndex :type Integer) (bFromSweep :type Boolean) (SweepResult :type Hit%20Result%20Structure%20%28by%20ref%29))
  (if (Variables|Default|Getm_bOpen)
    (if (not (Variables|Default|Getm_bSwingFront))
      (Collision|SetCollisionEnabled (Variables|Default|GetFront) "NoCollision" :!label _label)
      ;[1 1 1] Door Openning
      (bind (_direction _delta) (Timeline|DoorSwing Play)
        (:Update
          (Transformation|SetRelativeRotation (Variables|Default|GetDoor2) (Math|Rotator|MakeRotator 0.0 0.0 (* _delta (Variables|Default|Getm_fSwingRotTarget) (Math|Float|SelectFloat 1.0 -1.0 (Variables|Default|Getm_bSwingFront)))) true false)
          (Transformation|SetRelativeRotation (Variables|Default|GetDoor1) (* (Math|Rotator|MakeRotator 0.0 0.0 (* _delta (Variables|Default|Getm_fSwingRotTarget) (Math|Float|SelectFloat 1.0 -1.0 (Variables|Default|Getm_bSwingFront)))) -1.0) true false))
        (:Finished
          (if (Utilities|Enum|Equal(Enum) _direction "Backward")
            (Variables|Default|Setm_bOpen false)
            (Collision|SetCollisionEnabled (Variables|Default|GetFront) "QueryOnly")))))
    (else
      (Variables|Default|Setm_bSwingFront false)
      (Variables|Default|Setm_bOpen true)
      (goto _label))))

(event OnComponentEndOverlap(Back)
  (params (OverlappedComponent :type Primitive%20Component%20Object%20Reference) (OtherActor :type Actor%20Object%20Reference) (OtherComp :type Primitive%20Component%20Object%20Reference) (OtherBodyIndex :type Integer))
  ;[1 1 1] Door Openning
  (bind (_direction _delta) (Timeline|DoorSwing Reverse)
    (:Update
      (Transformation|SetRelativeRotation (Variables|Default|GetDoor2) (Math|Rotator|MakeRotator 0.0 0.0 (* _delta (Variables|Default|Getm_fSwingRotTarget) (Math|Float|SelectFloat 1.0 -1.0 (Variables|Default|Getm_bSwingFront)))) true false)
      (Transformation|SetRelativeRotation (Variables|Default|GetDoor1) (* (Math|Rotator|MakeRotator 0.0 0.0 (* _delta (Variables|Default|Getm_fSwingRotTarget) (Math|Float|SelectFloat 1.0 -1.0 (Variables|Default|Getm_bSwingFront)))) -1.0) true false))
    (:Finished
      (if (Utilities|Enum|Equal(Enum) _direction "Backward")
        (Variables|Default|Setm_bOpen false)
        (Collision|SetCollisionEnabled (Variables|Default|GetFront) "QueryOnly")))))

(fn ConstructionScript)